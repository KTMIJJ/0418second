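; BP_Body is a player-steered P38 aircraft that flies continuously forward along its local X axis.
; Each tick it offsets itself by its speed and spins the Left and Right propellers around their roll axis, all scaled by delta time.
; Pitch and Roll axis inputs are clamped and applied as local rotations, with both using PitchRotateSpeed as the turn rate.
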(event `self.ReceiveTick`
  (params (DeltaSeconds :type "Float (single-precision)"))
  (`self.K2_AddActorLocalOffset` (`KismetMathLibrary.MakeVector` (* (`GameplayStatics.GetWorldDeltaSeconds`) (`self.Speed/sec`))))
  (`SceneComponent.K2_AddRelativeRotation` (`self.Left`) (`KismetMathLibrary.MakeRotator` (* (`GameplayStatics.GetWorldDeltaSeconds`) (`self.PropellerSpeed`))) false false)
  (`SceneComponent.K2_AddRelativeRotation` (`self.Right`) (`KismetMathLibrary.MakeRotator` (* (`GameplayStatics.GetWorldDeltaSeconds`) (`self.PropellerSpeed`))) false false))

(event `InputAxis|Pitch`
  (params (AxisValue :type "Float (single-precision)"))
  (`self.K2_AddActorLocalRotation` (`KismetMathLibrary.MakeRotator` 0.0 (* (`GameplayStatics.GetWorldDeltaSeconds`) (`KismetMathLibrary.FClamp` AxisValue -1.0) (`self.PitchRotateSpeed`)))))

(event `InputAxis|Roll`
  (params (AxisValue :type "Float (single-precision)"))
  (`self.K2_AddActorLocalRotation` (`KismetMathLibrary.MakeRotator` (* (`GameplayStatics.GetWorldDeltaSeconds`) (`KismetMathLibrary.FClamp` AxisValue -1.0) (`self.PitchRotateSpeed`)))))

(fn `UserConstructionScript`)